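; BP_TreasureChest is an interactable world chest whose lid alternately opens and closes on each interaction.
; A FlipFlop plays or reverses the AnimLid timeline, which drives the lid mesh's pitch.
; CanInteract blocks further interaction until the timeline finishes, and GoldEffect activates once the lid has opened.
; A gameplay-tag keycard check against the action component exists but is disconnected, so the chest opens without one.
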(event `SGameplayInterface.Interact`
  (params (InstigatorPawn :type "Pawn Object Reference"))
  ;[1 1 1] Slowly open chest on interaction. Close it the second time. CanInteract makes sure that the lid closing/opening can't be spammed. Check if player has keycard before it can open the chest.
  (if (`self.CanInteract`)
    (set `self.CanInteract` false)
    (bind _isa (`/Engine/EditorBlueprintResources/StandardMacros.FlipFlop`)
      (:`A`
        (bind (_direction _pitch) (`Timeline|AnimLid` :!label _label)
          (:`Update`
            (`SceneComponent.K2_SetRelativeRotation` (`self.LidMesh`) (`KismetMathLibrary.MakeRotator` 0.0 _pitch) false false))
          (:`Finished`
            (set `self.CanInteract` true)
            (if _isa
              (`ActorComponent.Activate` (`self.GoldEffect`) false)))))
      (:`B`
        (goto _label :!via `Reverse`)))))

(fn `UserConstructionScript`)