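; BP_DashGrant is an interactable world object that grants a character Dash, described in its prompt as a one-time-use ability.
; On interaction, it adds the Status.Owns.Dash tag to the SCharacter action component's active gameplay tags, then disables itself, unless that tag is already present.
; GetInteractText checks the same tag to show either the offer or an already-owned message.
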(event `SGameplayInterface.Interact`
  (params (InstigatorPawn :type "Pawn Object Reference"))
  (bind _asscharacter (cast `SCharacter` InstigatorPawn))
  (bind _activegameplaytags (`SActionComponent.ActiveGameplayTags` (`SCharacter.ActionComp` _asscharacter)))
  (if (not (`BlueprintGameplayTagLibrary.HasTag` _activegameplaytags (struct :`TagName` "Status.Owns.Dash") true))
    (`BlueprintGameplayTagLibrary.AddGameplayTag` _activegameplaytags (struct :`TagName` "Status.Owns.Dash"))
    (`self.Disable`)))

(fn `GetInteractText`
  (params (InstigatorPawn :type "Pawn Object Reference"))
  (returns (ReturnValue :type Text))
  (bind _asscharacter (cast `SCharacter` InstigatorPawn))
  (if (`BlueprintGameplayTagLibrary.HasTag` (`SActionComponent.ActiveGameplayTags` (`SCharacter.ActionComp` _asscharacter)) (struct :`TagName` "Status.Owns.Dash") true)
    (return "Can't pickup Dash. You already have it available.")
    (else
      (return "Grants a one-time-use Dash Ability."))))

(fn `UserConstructionScript`)