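; BP_ProjectileCanon is a world-object cannon that automatically fires magic projectiles at a fixed interval.
; A looping timer started on BeginPlay spawns BP_MagicProjectile at the actor's location and rotation, passing along its DamageAmount.
; Each Tick turns the Arrow component toward the first player's pawn, while the spawn transform reads the actor's rotation rather than the Arrow's.
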(event `self.ReceiveBeginPlay`
  (`KismetSystemLibrary.K2_SetTimerDelegate` (delegate `OnTimerElapsed`) 2.0 true))

(event `OnTimerElapsed`
  (`|SpawnActorFromClass` "/Game/ActionRoguelike/Abilities/BP_MagicProjectile.BP_MagicProjectile_C" (`KismetMathLibrary.MakeTransform` (`self.K2_GetActorLocation`) (`self.K2_GetActorRotation`)) "Undefined" "MultiplyWithRoot" null (`self.DamageAmount`) null))

(event `self.ReceiveTick`
  (params (DeltaSeconds :type "Float (single-precision)"))
  (`SceneComponent.K2_SetWorldRotation` (`self.Arrow`) (`KismetMathLibrary.MakeRotFromX` (- (`self.K2_GetActorLocation` (`GameplayStatics.GetPlayerPawn` 0)) (`self.K2_GetActorLocation`))) false false))

(fn `UserConstructionScript`)