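; BP_BlackHole is a short-lived black hole ability actor that destroys physics-simulated objects it touches.
; On BeginPlay it sets a five-second lifespan and records the sphere component's starting height.
; Sphere overlaps destroy the other actor when the overlapping component simulates physics.
; Tick resets the sphere's Z to the recorded height, confining any movement to a horizontal plane.
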(event `self.ReceiveBeginPlay`
  ;[1 1 1] Record original Z location
  (`self.SetLifeSpan` 5.0)
  (set `self.Initial Z` (.z (`SceneComponent.K2_GetComponentLocation` (`self.SphereComp`)))))

(event `self.SphereComp.OnComponentBeginOverlap`
  (params (OverlappedComponent :type "PrimitiveComponent Object Reference") (OtherActor :type "Actor Object Reference") (OtherComp :type "PrimitiveComponent Object Reference") (OtherBodyIndex :type Integer) (bFromSweep :type Boolean) (SweepResult :type "HitResult Structure (by ref)"))
  ;[1 1 1] Destroy hit actor on hit
  (`/Engine/EditorBlueprintResources/StandardMacros.IsValid` OtherComp
    (:`Is Valid`
      (if (`SceneComponent.IsSimulatingPhysics` OtherComp "None")
        (`self.K2_DestroyActor` OtherActor)))))

(event `self.ReceiveTick`
  (params (DeltaSeconds :type "Float (single-precision)"))
  ;[1 1 1] Set Z location
  (`SceneComponent.K2_SetWorldLocation` (`self.SphereComp`) (`KismetMathLibrary.MakeVector` (.x (`SceneComponent.K2_GetComponentLocation` (`self.SphereComp`))) (.y (`SceneComponent.K2_GetComponentLocation` (`self.SphereComp`))) (`self.Initial Z`)) false false))

(fn `UserConstructionScript`)